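; BP_PawnBase is a base pawn that glides and banks in response to movement input.
; On BeginPlay it binds to the OnUpdateMove dispatcher of BP_PlayerControllerBase to store the incoming move vector.
; Each Tick it eases a movement offset toward that vector times speed, then applies it as a swept, per-frame step unscaled by delta time.
; The offset's Y component drives an interpolated roll tilt, with pitch and yaw targeting zero.
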(event `self.ReceiveBeginPlay`
  (bind _returnvalue (`GameplayStatics.GetActorOfClass` "/Game/Blueprints/PlayerControllers/BP_PlayerControllerBase.BP_PlayerControllerBase_C"))
  (add `/Game/Blueprints/PlayerControllers/BP_PlayerControllerBase.OnUpdateMove` _returnvalue (delegate `OnUpdateMove_Event`)))

(event `OnUpdateMove_Event`
  (params (NewParam :type "Vector Structure"))
  (`self.UpdateMoveVector` NewParam))

(event `self.ReceiveTick`
  (params (DeltaSeconds :type "Float (single-precision)"))
  (bind (_returnvalue_x _returnvalue_y) (`KismetMathLibrary.BreakVector` (* (`self.CurrentVector`) (`self.TiltFactor`))))
  (set `self.TargetVector` (* (`self.MoveVector`) (`self.MovementSpeed`)))
  (bind _output_get (set `self.CurrentVector` (`KismetMathLibrary.VInterpTo` (`self.CurrentVector`) (`self.TargetVector`) (`GameplayStatics.GetWorldDeltaSeconds`) (`self.MovementInterpSpeed`))))
  (`self.K2_SetActorLocationAndRotation` (+ _output_get (`self.K2_GetActorLocation`)) (`KismetMathLibrary.RInterpTo` (`self.K2_GetActorRotation`) (`KismetMathLibrary.MakeRotator` _returnvalue_y) (`GameplayStatics.GetWorldDeltaSeconds`) (`self.RotationInterpSpeed`)) true))

(fn `UpdateMoveVector`
  (params (MoveVector :type "Vector Structure"))
  (set `self.MoveVector` MoveVector))

(fn `UserConstructionScript`)