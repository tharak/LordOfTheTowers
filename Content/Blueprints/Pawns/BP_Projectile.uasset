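; BP_Projectile is a projectile that moves on its own and expends itself on impact.
; On BeginPlay it gives its movable component a constant +X move vector.
; The first mesh hit on anything other than its owner adds a Niagara effect and applies its full current health as damage to its own health component.
; This graph applies no damage to the actor it hits.
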(event `self.ReceiveBeginPlay`
  (set `/Game/Blueprints/Components/BP_MovableComponent.MoveVector` (1.0 0.0 0.0) (`self.BP_MovableComponent`)))

(event `self.SM_Projectile.OnComponentHit`
  (params (HitComponent :type "PrimitiveComponent Object Reference") (OtherActor :type "Actor Object Reference") (OtherComp :type "PrimitiveComponent Object Reference") (NormalImpulse :type "Vector Structure") (Hit :type "HitResult Structure (by ref)"))
  (bind _bp_healthcomponent (`self.BP_HealthComponent`))
  (bind _health (`/Game/Blueprints/Components/BP_HealthComponent.Health` _bp_healthcomponent))
  (if (not (== OtherActor (`self.GetOwner`)))
    (`/Engine/EditorBlueprintResources/StandardMacros.DoOnce` false
      (:`Completed`
        (`AddComponent|NODE_AddNiagaraComponent-1`)
        (`/Game/Blueprints/Components/BP_HealthComponent.AnyDamage` _bp_healthcomponent _health null null null _health)))))

(fn `UserConstructionScript`)