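; BP_PawnPlayer is the player pawn, which moves and shoots in response to events from the player controller.
; On BeginPlay it finds a BP_PlayerControllerBase actor, binds to its move-vector and shoot dispatchers, and sets itself as the shooter component's owner.
; Move updates are passed to the movable component, and shoot events fire the shooter component from the projectile spawn point's world transform.
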(event `self.ReceiveBeginPlay`
  (bind _returnvalue (`GameplayStatics.GetActorOfClass` "/Game/Blueprints/PlayerControllers/BP_PlayerControllerBase.BP_PlayerControllerBase_C"))
  (bind _output_get (set `self.PlayerController` _returnvalue))
  (add `/Game/Blueprints/PlayerControllers/BP_PlayerControllerBase.OnPlayerUpdateMoveVector` _output_get (delegate `EventUpdatePlayerLocationAndRotation`))
  (add `/Game/Blueprints/PlayerControllers/BP_PlayerControllerBase.OnPlayerShoot` (`self.PlayerController`) (delegate `EventPlayerShoot`))
  (set `/Game/Blueprints/Components/BP_ShooterComponent.Owner` self (`self.BP_ShooterComponent`)))

(event `EventUpdatePlayerLocationAndRotation`
  (params (position :type "Vector Structure"))
  (`self.SetMoveVector` position))

(event `EventPlayerShoot`
  (`self.PlayerShoot`))

(event `self.ReceiveTick`
  (params (DeltaSeconds :type "Float (single-precision)")))

(fn `PlayerShoot`
  (`/Game/Blueprints/Components/BP_ShooterComponent.Shoot` (`self.BP_ShooterComponent`) (`SceneComponent.K2_GetComponentToWorld` (`self.ProjectileSpawnPoint`))))

(fn `SetMoveVector`
  (params (MoveVector :type "Vector Structure"))
  (set `/Game/Blueprints/Components/BP_MovableComponent.MoveVector` MoveVector (`self.BP_MovableComponent`)))

(fn `UserConstructionScript`)