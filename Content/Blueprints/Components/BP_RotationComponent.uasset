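; Rotation component that tilts its owning actor's root component according to a movement vector.
; Each tick it smooths CurrentRotation toward MoveVector times MovementSpeed, then maps its Y and Z, scaled by TiltFactor, to roll and pitch.
; That tilt, rather than the root's existing rotation, is interpolated one step toward TargetRotation and applied as relative rotation.
; MoveVector and TargetRotation are only read here, never set.
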(event `self.ReceiveBeginPlay`)

(event `self.ReceiveTick`
  (params (DeltaSeconds :type "Float (single-precision)"))
  (bind (_currentrotation_x _currentrotation_y _currentrotation_z) (`KismetMathLibrary.BreakVector` (`self.CurrentRotation`)))
  (bind (_returnvalue_x _returnvalue_y _returnvalue_z) (`KismetMathLibrary.BreakVector` (* (`KismetMathLibrary.MakeVector` _currentrotation_y _currentrotation_z) (`self.TiltFactor`))))
  (set `self.CurrentRotation` (`KismetMathLibrary.VInterpTo` (`self.CurrentRotation`) (* (`self.MoveVector`) (`self.MovementSpeed`)) (`GameplayStatics.GetWorldDeltaSeconds`) (`self.MovementInterpSpeed`)))
  (`SceneComponent.K2_SetRelativeRotation` (`Actor.RootComponent` (`self.GetOwner`)) (`KismetMathLibrary.RInterpTo` (`KismetMathLibrary.MakeRotator` _returnvalue_x _returnvalue_y _returnvalue_z) (`self.TargetRotation`) (`GameplayStatics.GetWorldDeltaSeconds`) (`self.RotationInterpSpeed`)) false false))