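; BP_HealthComponent is a health component that tracks damage taken and destroys its owning actor when health runs out.
; Its AnyDamage event subtracts the damage from Health and clamps the result between zero and a MaxHealth value passed into the event.
; At zero it prints a death message with the component's display name and destroys the owner, otherwise it prints the remaining health.
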(event `AnyDamage`
  (params (Damage :type "Float (double-precision)") (DamageTyoe :type "DamageType Object Reference") (InstigatedBy :type "Controller Object Reference") (DamageCauser :type "Actor Object Reference") (MaxHealth :type "Float (double-precision)"))
  (bind _output_get (set `self.Health` (`KismetMathLibrary.FClamp` (- (`self.Health`) Damage) 0.0 MaxHealth)))
  (if (<= _output_get 0.0)
    (`KismetSystemLibrary.PrintString` (`KismetStringLibrary.Concat_StrStr` "DEAD " (`KismetSystemLibrary.GetDisplayName` self)))
    (`Actor.K2_DestroyActor` (`self.GetOwner`))
    (else
      (`KismetSystemLibrary.PrintString` (`KismetStringLibrary.Conv_DoubleToString` (`self.Health`))))))