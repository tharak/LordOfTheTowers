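; Movable component that moves its owning actor along a MoveVector with smoothed speed changes.
; Each tick, CurrentLocation interpolates toward MoveVector times MovementSpeed, acting as a per-frame offset despite its name.
; That offset is added to the owner's location with sweep enabled, so blocking collision applies.
; The step itself is not scaled by delta time, so travel speed depends on frame rate.
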(event `self.ReceiveBeginPlay`
  (set `self.Owner` (`self.GetOwner`)))

(event `self.ReceiveTick`
  (params (DeltaSeconds :type "Float (single-precision)"))
  (bind _output_get (set `self.CurrentLocation` (`KismetMathLibrary.VInterpTo` (`self.CurrentLocation`) (* (`self.MoveVector`) (`self.MovementSpeed`)) (`GameplayStatics.GetWorldDeltaSeconds`) (`self.MovementInterpSpeed`))))
  (`Actor.K2_SetActorLocation` (`self.Owner`) (+ _output_get (`Actor.K2_GetActorLocation` (`self.Owner`))) true false))