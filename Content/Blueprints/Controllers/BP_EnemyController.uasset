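; BP_EnemyController is an enemy spawner that moves back and forth along the Y axis, creating BP_PawnEnemy actors.
; SetMoveDirection feeds MoveVectorY into BPMovableComponent at BeginPlay and after each bounce.
; When its Box hits a BlockingVolume, it reverses direction, waits a short random delay, then spawns an enemy using the location and scale of SpawnPoint.
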(event `self.ReceiveBeginPlay`
  (`self.SetMoveDirection`))

(event `self.ReceiveTick`
  (params (DeltaSeconds :type "Float (single-precision)")))

(event `self.Box.OnComponentHit`
  (params (HitComponent :type "PrimitiveComponent Object Reference") (OtherActor :type "Actor Object Reference") (OtherComp :type "PrimitiveComponent Object Reference") (NormalImpulse :type "Vector Structure") (Hit :type "HitResult Structure (by ref)"))
  (if (== (`GameplayStatics.GetObjectClass` OtherActor) "/Script/Engine.BlockingVolume")
    (set `self.Move Vector Y` (* (`self.Move Vector Y`) -1.0))
    (`self.SetMoveDirection`)
    (`KismetSystemLibrary.Delay` (`KismetMathLibrary.RandomFloatInRange` 0.5 2.5))
    (`self.SpawnEnemy`)))

(fn `SetMoveDirection`
  (set `/Game/Blueprints/Components/BP_MovableComponent.MoveVector` (`KismetMathLibrary.MakeVector` 0.0 (`self.Move Vector Y`)) (`self.BP_MovableComponent`)))

(fn `SpawnEnemy`
  (bind (_returnvalue_location _returnvalue_rotation _returnvalue_scale) (`KismetMathLibrary.BreakTransform` (`SceneComponent.K2_GetComponentToWorld` (`self.SpawnPoint`))))
  (`|SpawnActorFromClass` "/Game/Blueprints/Pawns/BP_PawnEnemy.BP_PawnEnemy_C" (`KismetMathLibrary.MakeTransform` _returnvalue_location (struct) _returnvalue_scale) "AlwaysSpawn" "MultiplyWithRoot" null null))

(fn `UserConstructionScript`)