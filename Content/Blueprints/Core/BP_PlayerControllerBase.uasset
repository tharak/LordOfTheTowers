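; BP_PlayerControllerBase is the base player controller that routes Enhanced Input to the player pawn.
; On BeginPlay it adds the IMC_Main mapping context and caches the first BP_PawnBase found in the level.
; IA_Move sends the delta-time-scaled input as a Y-only move vector to that pawn and zeroes it on completion.
; Fire, restart and set-destination input events are empty stubs.
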(event `self.ReceiveBeginPlay`
  (`EnhancedInputSubsystemInterface.AddMappingContext` (pcsubsystem `EnhancedInputLocalPlayerSubsystem` (`GameplayStatics.GetPlayerController` 0)) "/Game/Input/IMC_Main.IMC_Main" 0 (struct))
  (bind _returnvalue (`GameplayStatics.GetActorOfClass` "/Game/Blueprints/Core/BP_PawnBase.BP_PawnBase_C"))
  (set `self.PlayerPawn` _returnvalue))

(event `EnhancedInput|/Game/Input/IA_Fire`
  (params (ActionValue :type Boolean) (ElapsedSeconds :type "Float (double-precision)") (TriggeredSeconds :type "Float (double-precision)") (InputAction :type "InputAction Object Reference" :default "/Game/Input/IA_Fire.IA_Fire")))

(event `EnhancedInput|/Game/Input/IA_Move`
  (params (ActionValue :type "Float (double-precision)") (ElapsedSeconds :type "Float (double-precision)") (TriggeredSeconds :type "Float (double-precision)") (InputAction :type "InputAction Object Reference" :default "/Game/Input/IA_Move.IA_Move"))
  (bind _playerpawn (`self.PlayerPawn`))
  (:`Triggered`
    (`/Game/Blueprints/Core/BP_PawnBase.UpdateMoveVector` _playerpawn (`KismetMathLibrary.MakeVector` 0.0 (* (`GameplayStatics.GetWorldDeltaSeconds`) ActionValue))))
  (:`Completed`
    (`/Game/Blueprints/Core/BP_PawnBase.UpdateMoveVector` _playerpawn (0.0 0.0 0.0))))

(event `EnhancedInput|/Game/Input/IA_Restart`
  (params (ActionValue :type Boolean) (ElapsedSeconds :type "Float (double-precision)") (TriggeredSeconds :type "Float (double-precision)") (InputAction :type "InputAction Object Reference" :default "/Game/Input/IA_Restart.IA_Restart")))

(event `EnhancedInput|/Game/ThirdParty/TopDown/Input/Actions/IA_SetDestination_Click`
  (params (ActionValue :type Boolean) (ElapsedSeconds :type "Float (double-precision)") (TriggeredSeconds :type "Float (double-precision)") (InputAction :type "InputAction Object Reference" :default "/Game/ThirdParty/TopDown/Input/Actions/IA_SetDestination_Click.IA_SetDestination_Click")))

(event `EnhancedInput|/Game/ThirdParty/TopDown/Input/Actions/IA_SetDestination_Touch`
  (params (ActionValue :type Boolean) (ElapsedSeconds :type "Float (double-precision)") (TriggeredSeconds :type "Float (double-precision)") (InputAction :type "InputAction Object Reference" :default "/Game/ThirdParty/TopDown/Input/Actions/IA_SetDestination_Touch.IA_SetDestination_Touch")))

(fn `UserConstructionScript`)