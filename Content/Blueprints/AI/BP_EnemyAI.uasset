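; BP_EnemyAI is an enemy actor that moves, rotates, shoots and is destroyed when hit by a projectile it does not own.
; SetMoveDirection feeds its movable and rotation components, and FireWeapon spawns shots ahead of it through the shooter component.
; SetAlertVisual tints a dynamic material red at once, then clears it after a short timer delay, which a renewed alert cancels.
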(event `self.ReceiveBeginPlay`
  (bind _returnvalue (`PrimitiveComponent.CreateDynamicMaterialInstance` (`self.StaticMesh`) 0 null "None"))
  (set `self.AlertMaterial` _returnvalue))

(event `self.SetAlertVisual`
  (params (bAlert :type Boolean))
  (if bAlert
    (`KismetSystemLibrary.K2_ClearTimer` null "ApplyAlertOff")
    (`MaterialInstanceDynamic.SetVectorParameterValue` (`self.AlertMaterial`) "TextureColour" (struct :`R` 1.0 :`A` 1.0))
    (`MaterialInstanceDynamic.SetScalarParameterValue` (`self.AlertMaterial`) "ColourMask" 1.0)
    (else
      (`KismetSystemLibrary.K2_SetTimer` null "ApplyAlertOff" 1.5))))

(event `ApplyAlertOff`
  (`MaterialInstanceDynamic.SetVectorParameterValue` (`self.AlertMaterial`) "TextureColour" (struct :`A` 1.0))
  (`MaterialInstanceDynamic.SetScalarParameterValue` (`self.AlertMaterial`) "ColourMask" 0.0))

(event `self.SetMoveDirection`
  (params (Direction :type "Vector Structure (by ref)"))
  (set `/Game/Blueprints/Components/BP_MovableComponent.MoveVector` Direction (`self.BP_MovableComponent`))
  (set `/Game/Blueprints/Components/BP_RotationComponent.MoveVector` Direction (`self.BP_RotationComponent`)))

(event `self.StaticMesh.OnComponentHit`
  (params (HitComponent :type "PrimitiveComponent Object Reference") (OtherActor :type "Actor Object Reference") (OtherComp :type "PrimitiveComponent Object Reference") (NormalImpulse :type "Vector Structure") (Hit :type "HitResult Structure (by ref)"))
  (bind _asbp_projectile (cast `/Game/Blueprints/Pawns/BP_Projectile` OtherActor))
  (if (!= (`self.GetOwner` _asbp_projectile) self)
    (`self.K2_DestroyActor`)))

(event `self.FireWeapon`
  (`/Game/Blueprints/Components/BP_ShooterComponent.Shoot` (`self.BP_ShooterComponent`) (`KismetMathLibrary.MakeTransform` (+ (`self.K2_GetActorLocation`) (* (`self.GetActorForwardVector`) (105.0 105.0 105.0))) (`self.K2_GetActorRotation`)))
  (`KismetSystemLibrary.PrintString` "SHOOT"))

(fn `UserConstructionScript`)